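; BP_PJ_Principal is the main character actor, which moves itself every Tick along its normalized Direccion vector.
; The step is FactorVelocidad times VelocidadBase, applied as a world offset without sweep or delta-time scaling.
; Each Tick also fetches all BP_Enemigo actors, copies the attacking flag of index 1 into EstaSiendoAtacado, and sets the speed factor to a fixed value.
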(event EventTick
  (params (DeltaSeconds :type Float%20%28single-precision%29))
  (Transformation|AddActorWorldOffset (* (Math|Vector|Normalize (Variables|Components|GetDireccion)) (* (Variables|Components|GetFactorVelocidad) (Variables|Components|GetVelocidadBase))))
  (bind _outactors (Actor|GetAllActorsOfClass "/Game/Enemigo/BP_Enemigo.BP_Enemigo_C"))
  (Variables|Components|SetEstaSiendoAtacado (Variables|/Game/Enemigo/BP_Enemigo.BP_Enemigo_C|GetEstaAtacandoVar? (Utilities|Array|Get(acopy) _outactors 1)))
  (Variables|Components|SetFactorVelocidad 2.0))

(fn ConstructionScript)