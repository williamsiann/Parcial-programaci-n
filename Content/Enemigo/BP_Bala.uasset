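; BP_Bala is an enemy bullet that homes in on the player character, BP_PJ_Principal.
; Each Tick it finds all player actors and moves toward each by the normalized direction times Velocidad, without sweep or delta-time scaling.
; A Delay inside the same loop destroys the bullet five seconds after it first finds a player.
; The graph contains no hit or damage logic.
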(event EventTick
  (params (DeltaSeconds :type Float%20%28single-precision%29))
  (bind _outactors (Actor|GetAllActorsOfClass "/Game/BP_PJ_Principal.BP_PJ_Principal_C"))
  (for _array_element _outactors
    (Variables|Components|SetUbicacion (Math|Vector|Normalize (- (Transformation|GetActorLocation _array_element) (Transformation|GetActorLocation))))
    (Transformation|AddActorWorldOffset (* (Math|Vector|Normalize (- (Transformation|GetActorLocation _array_element) (Transformation|GetActorLocation))) (Variables|Components|GetVelocidad)))
    (Utilities|FlowControl|Delay 5.0)
    (Actor|DestroyActor)))

(fn ConstructionScript)